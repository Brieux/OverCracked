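; BP_Cam is a camera actor that becomes the player's view target on BeginPlay and provides shake and drug-trip screen effects.
; CamShake plays BP_CamShake at the camera's location.
; DrugEffect toggles via FlipFlop: a speed-adjusted timeline drives FOV, effect intensity and red-channel saturation, offset by a random start value and wrapped.
; Toggling off stops the timeline and zeroes intensity without explicitly restoring FOV.
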(event `self.ReceiveBeginPlay`
  (set `self.RandomHue` (`KismetMathLibrary.RandomFloatInRange` 0.0 1.0))
  (`PlayerController.SetViewTargetWithBlend` (`GameplayStatics.GetPlayerController` 0) self 0.0 "VTBlend_Linear" 0.0 false))

(event `CamShake`
  (`GameplayStatics.PlayWorldCameraShake` "/Game/BP_CamShake.BP_CamShake_C" (`self.K2_GetActorLocation`) 0.0 1.0))

(event `DrugEffect`
  (bind _camera (`self.Camera`))
  (`/Engine/EditorBlueprintResources/StandardMacros.FlipFlop`
    (:`A`
      (`TimelineComponent.SetPlayRate` (`self.Timeline_0`) (`self.SpeedDrug`))
      (bind (_direction _newtrack_0) (`Timeline|Timeline_0` :!label _label)
        (:`Update`
          (set `CameraComponent.PostProcessSettings` (make `PostProcessSettings` :`ColorSaturation` (`KismetMathLibrary.MakeVector4` (mod (+ (`self.RandomHue`) _newtrack_0) 1.0) 1.0 1.0 1.0) :`SceneFringeIntensity` (* _newtrack_0 6.0)) _camera)
          (`CameraComponent.SetFieldOfView` _camera (`KismetMathLibrary.Lerp` 87.0 92.0 _newtrack_0)))))
    (:`B`
      (`|ExecutionSequence`
        (:`then_0`
          (goto _label :!via `Stop`))
        (:`then_1`
          (set `CameraComponent.PostProcessSettings` (make `PostProcessSettings`) (`self.Camera`)))))))

(fn `UserConstructionScript`)