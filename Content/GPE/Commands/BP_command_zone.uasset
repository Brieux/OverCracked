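; Command zone that serves as the order counter where dropped syringes are checked against timed ingredient recipes for score.
; A looping timer adds random one-to-three-ingredient orders, up to three queued, while another drains their patience and removes expired ones.
; Box overlap checks syringe contents regardless of ingredient order, then destroys it.
; The check stops at the first order, either scoring time times challenge or docking its time.
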(event `DropSyringe`
  (params (SyringeDropped :type "/Game/GPE/Commands/BP_Syringe Object Reference"))
  (bind _commandlist (`self.CommandList`))
  (bind (_recipe _time _challenge) (break `/Game/GPE/Commands/STRUCT_command` (`|GetArrayItem` _commandlist)))
  (`KismetSystemLibrary.PrintString` "BeginScan" true true (struct :`R` 0.276319 :`G` 1.0 :`A` 1.0) 5.0)
  (for (_array_element _array_index) (`self.CommandList`)
    (bind (_recipe_2 _time_2) (break `/Game/GPE/Commands/STRUCT_command` _array_element))
    (if (== (`KismetArrayLibrary.Array_Length` _recipe_2) (`KismetArrayLibrary.Array_Length` (`/Game/GPE/Commands/BP_Syringe.Content` SyringeDropped)))
      (set `self.CheckIngredients` true)
      (for _array_element_2 _recipe_2
        (if (not (`KismetArrayLibrary.Array_Contains` (`/Game/GPE/Commands/BP_Syringe.Content` SyringeDropped) _array_element_2))
          (set `self.CheckIngredients` false)
          (break)))
      (if (`self.CheckIngredients`)
        (set `self.Validated` true)
        (set `self.RemovedIndex` _array_index)
        (break)
        (else
          _)))
    ;[1 1 1] Wrong recipe
    (bind _structout (setmembers `/Game/GPE/Commands/STRUCT_command` :`StructRef` _array_element :`Time` (- _time_2 5.0)))
    (`KismetArrayLibrary.Array_Set` _commandlist _array_index _structout)
    (set `self.Validated` false)
    ;[1 1 1] FailureFeedback
    (`KismetSystemLibrary.PrintString` "NOT THE RIGHT RECIPE : -5")
    (break))
  (if (`self.Validated`)
    (set `self.Score` (+ (`self.Score`) (* _time _challenge)))
    ;[1 1 1] SuccessFeedback
    (`KismetSystemLibrary.PrintString` "Congratulation" true true (struct :`R` 1.0 :`G` 0.020908 :`A` 1.0) 20.0)
    (`KismetArrayLibrary.Array_Remove` _commandlist (`self.RemovedIndex`))
    (set `self.RemovedIndex` 0)))

(event `self.ReceiveBeginPlay`
  (`KismetSystemLibrary.K2_SetTimerDelegate` (delegate `LoosePatience`) 1.0 true)
  (`KismetSystemLibrary.K2_SetTimerDelegate` (delegate `GenerateCommand`) 10.0 true))

(event `GenerateCommand`
  (bind _newparam (`self.RandomIngredientGeneration`))
  (bind _newparam_2 (`self.RandomIngredientGeneration`))
  (bind _returnvalue (`KismetMathLibrary.RandomFloatInRange` 30.0 60.0))
  (bind _returnvalue_2 (`KismetMathLibrary.RandomFloat`))
  (bind _returnvalue_3 (> _returnvalue_2 0.4))
  (bind _returnvalue_4 (> _returnvalue_2 0.7))
  (bind _returnvalue_5 (- (+ _returnvalue (`KismetMathLibrary.SelectFloat` 10.0 0.0 _returnvalue_3) (`KismetMathLibrary.SelectFloat` 20.0 0.0 _returnvalue_4)) (`KismetMathLibrary.FMod` _returnvalue 5.0)))
  (if (< (`KismetArrayLibrary.Array_Length` (`self.CommandList`)) 3)
    (`KismetArrayLibrary.Array_Add` (`self.CommandList`) (make `/Game/GPE/Commands/STRUCT_command` (select `bool` _returnvalue_3 :`false` (`|MakeArray` _newparam) :`true` (select `bool` _returnvalue_4 :`false` (`|MakeArray` _newparam _newparam_2) :`true` (`|MakeArray` _newparam _newparam_2 (`self.RandomIngredientGeneration`)))) _returnvalue_5 (select `bool` _returnvalue_3 :`false` 1 :`true` (select `bool` _returnvalue_4 :`false` 2 :`true` 3))))
    (`self.NewRecipes`)
    (`KismetSystemLibrary.PrintString` (`KismetStringLibrary.Conv_DoubleToString` _returnvalue_5))))

(event `LoosePatience`
  (`|ExecutionSequence`
    (:`then_0`
      (`self.PatienceLost`))
    (:`then_1`
      (`KismetSystemLibrary.PrintString` (`KismetStringLibrary.Conv_IntToString` (`KismetArrayLibrary.Array_Length` (`self.CommandList`)))))))

(event `self.Box.OnComponentBeginOverlap`
  (params (OverlappedComponent :type "PrimitiveComponent Object Reference") (OtherActor :type "Actor Object Reference") (OtherComp :type "PrimitiveComponent Object Reference") (OtherBodyIndex :type Integer) (bFromSweep :type Boolean) (SweepResult :type "HitResult Structure (by ref)"))
  (`/Engine/EditorBlueprintResources/StandardMacros.DoOnce` false :!label _label
    (:`Completed`
      (bind _asbp_syringe (cast `/Game/GPE/Commands/BP_Syringe` OtherActor)
        (:`then`
          (`self.DropSyringe` _asbp_syringe)
          ;[1 1 1] Animation
          (`KismetSystemLibrary.Delay` 1.0)
          (`self.K2_DestroyActor` _asbp_syringe)
          (goto _label :!via `Reset`))
        (:`CastFailed`
          (goto _label :!via `Reset`))))))

(fn `RandomIngredientGeneration`
  (returns (NewParam :type "/Game/Struct_Ingredient Structure"))
  (return (make `/Game/Struct_Ingredient` (select `int` (`KismetMathLibrary.RandomInteger` 3) :`0` "NewEnumerator0" :`1` "NewEnumerator1" :`2` "NewEnumerator2" :!type "/Game/enum_color Enum") (select `int` (`KismetMathLibrary.RandomInteger` 3) :`0` "NewEnumerator0" :`1` "NewEnumerator1" :`2` "NewEnumerator2" :!type "/Game/Enum_State Enum"))))

(fn `UserConstructionScript`)