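; Syringe gameplay actor that holds a single ingredient as its content.
; On BeginPlay it caches both players' top-down character pawns, printing an error if either cast fails.
; AddIngredient stores only the first ingredient received through a DoOnce, and Ciao destroys the actor.
; The PlayerDetection overlap compares the actor to both players but triggers no action yet.
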(event `self.ReceiveBeginPlay`
  (bind _asbp_top_down_character (cast `/Game/TopDown/Blueprints/BP_TopDownCharacter` (`GameplayStatics.GetPlayerPawn` 0))
    (:`then`
      (set `self.Player1Pawn` _asbp_top_down_character)
      (bind _asbp_top_down_character_2 (cast `/Game/TopDown/Blueprints/BP_TopDownCharacter` (`GameplayStatics.GetPlayerPawn` 1))
        (:`then`
          (set `self.Player2Pawn` _asbp_top_down_character_2))
        (:`CastFailed`
          (`KismetSystemLibrary.PrintString` "ERROR :::::::: NOT CORRECT TYPE" true true (struct :`G` 0.66 :`B` 1.0 :`A` 1.0) 10000.0 :!label _label))))
    (:`CastFailed`
      (goto _label))))

(event `AddIngredient`
  (params (IngredientAdded :type "Array of /Game/Struct_Ingredient Structure"))
  (`/Engine/EditorBlueprintResources/StandardMacros.DoOnce` false
    (:`Completed`
      (set `self.Content` IngredientAdded))))

(event `self.PlayerDetection.OnComponentBeginOverlap`
  (params (OverlappedComponent :type "PrimitiveComponent Object Reference") (OtherActor :type "Actor Object Reference") (OtherComp :type "PrimitiveComponent Object Reference") (OtherBodyIndex :type Integer) (bFromSweep :type Boolean) (SweepResult :type "HitResult Structure (by ref)"))
  (if (== OtherActor (`self.Player1Pawn`))
    _
    (elif (== OtherActor (`self.Player2Pawn`))
      _)))

(event `/Game/GPE/BPI_Grabbable.Ciao`
  (`self.K2_DestroyActor`))

(fn `UserConstructionScript`)