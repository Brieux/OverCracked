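; BP_Ingredient is a mixable-component ingredient with a color and texture, stored in a STRUCTIngredient.
; The construction script derives red, blue or green from GeneratorType, applies the matching cylinder material, and randomly picks liquid, dust or solid texture on each run.
; Shake plays a texture-specific prototype 2D sound, throttled by a DoOnce that resets after a short delay.
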(event `Shake`
  (`/Engine/EditorBlueprintResources/StandardMacros.DoOnce` false :!label _label
    (:`Completed`
      (`GameplayStatics.SpawnSound2D` (select `/Game/GPE/MixableCOmponents/ENUM_Ingredient_Textures` (`.Texture_5_6617630347BF2BC424C4EC8BFD6A57DE` (break `/Game/GPE/MixableCOmponents/STRUCT_Ingredient` (`self.Type`))) :`NewEnumerator0` "/Game/Sounds/IngredientsSound/PROTOTYPE_1.PROTOTYPE_1" :`NewEnumerator1` "/Game/Sounds/IngredientsSound/PROTOTYPE_2.PROTOTYPE_2" :`NewEnumerator2` "/Game/Sounds/IngredientsSound/PROTOTYPE_3.PROTOTYPE_3" :!type "SoundBase Object Reference") 1.0 1.0 0.0 null)
      (`KismetSystemLibrary.Delay` 0.2)
      (goto _label :!via `Reset`))))

(fn `UserConstructionScript`
  (bind _returnvalue (select `int` (`self.GeneratorType`) :`0` "NewEnumerator0" :`1` "NewEnumerator1" :`2` "NewEnumerator2" :!type "/Game/GPE/MixableCOmponents/ENUM_ingredient_color Enum"))
  (set `self.Type` (make `/Game/GPE/MixableCOmponents/STRUCT_Ingredient` _returnvalue (select `int` (`KismetMathLibrary.RandomInteger` 3) :`0` "NewEnumerator0" :`1` "NewEnumerator1" :`2` "NewEnumerator2" :!type "/Game/GPE/MixableCOmponents/ENUM_Ingredient_Textures Enum")))
  (`PrimitiveComponent.SetMaterial` (`self.Cylinder`) 0 (select `/Game/GPE/MixableCOmponents/ENUM_ingredient_color` _returnvalue :`NewEnumerator0` "/Game/Material/MAT_IngredientRed.MAT_IngredientRed" :`NewEnumerator1` "/Game/Material/MAT_IngredientBlue.MAT_IngredientBlue" :`NewEnumerator2` "/Game/Material/MAT_IngredientGreen.MAT_IngredientGreen" :!type "MaterialInterface Object Reference")))