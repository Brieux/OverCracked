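; BP_IngredientSpawner is a placeable spawner that keeps one BP_Ingredient of a configured color (red, green or blue) available at its spawn point.
; It spawns shortly after BeginPlay, binds to the ingredient's Collected event, and respawns after a delay once it is collected.
; A failed spawn retries through the same refill path.
; The construction script tints one skeletal mesh material slot to match the chosen color.
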(event `self.ReceiveBeginPlay`
  (`KismetSystemLibrary.Delay` 0.2)
  (`self.SpawnIngredient`))

(event `SpawnIngredient`
  (bind _returnvalue (`|SpawnActorFromClass` "/Game/BP_Ingredient.BP_Ingredient_C" (`SceneComponent.K2_GetComponentToWorld` (`self.SpawnPoint`)) "Undefined" "OverrideRootScale" null (select `/Game/enum_color` (`self.Type`) :`NewEnumerator1` 1 :`NewEnumerator2` 2) 0 null))
  (if (`KismetSystemLibrary.IsValid` _returnvalue)
    (bind _output_get (set `self.CurrentItem` _returnvalue))
    (add `/Game/BP_Ingredient.Collected` _output_get (delegate `RefillIngredients`))
    (else
      (`KismetSystemLibrary.Delay` 0.25)
      (`self.RefillIngredients`))))

(event `RefillIngredients`
  (remove `/Game/BP_Ingredient.Collected` (`self.CurrentItem`) (delegate `RefillIngredients`))
  (set `self.CurrentItem` null)
  (`KismetSystemLibrary.Delay` 2.0)
  (`self.SpawnIngredient`))

(fn `UserConstructionScript`
  (`PrimitiveComponent.SetMaterial` (`self.SkeletalMesh`) 2 (select `/Game/enum_color` (`self.Type`) :`NewEnumerator0` "/Game/Material/MasterMaterial_FlatShading_Red.MasterMaterial_FlatShading_Red" :`NewEnumerator1` "/Game/Material/MasterMaterial_FlatShading_Green.MasterMaterial_FlatShading_Green" :`NewEnumerator2` "/Game/Material/MasterMaterial_FlatShading_DarkBlue.MasterMaterial_FlatShading_DarkBlue" :!type "MaterialInterface Object Reference")))