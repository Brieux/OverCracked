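; BP_MixingMachine is a machine that mixes ingredients and loads the mix into a syringe.
; Ingredients entering its box are destroyed, with up to three stored and shown as red, green or blue materials on indicator meshes.
; When a syringe enters a non-empty, unoccupied machine, it is detached and locked at the arrow.
; A timer then copies the mix into the syringe and resets the machine.
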(event `self.Box.OnComponentBeginOverlap`
  (params (OverlappedComponent :type "PrimitiveComponent Object Reference") (OtherActor :type "Actor Object Reference") (OtherComp :type "PrimitiveComponent Object Reference") (OtherBodyIndex :type Integer) (bFromSweep :type Boolean) (SweepResult :type "HitResult Structure (by ref)"))
  (bind _asbp_ingredient (cast `/Game/BP_Ingredient` OtherActor)
    (:`then`
      (if (< (`KismetArrayLibrary.Array_Length` (`self.MixedIngredients`)) 3)
        (bind _struct_type_obj (`/Game/BP_Ingredient.struct_type_obj` _asbp_ingredient))
        (`KismetArrayLibrary.Array_Add` (`self.MixedIngredients`) _struct_type_obj)
        (`PrimitiveComponent.SetMaterial` (select `int` (- (`KismetArrayLibrary.Array_Length` (`self.MixedIngredients`)) 1) :`0` (`self.COLOR1`) :`1` (`self.COLOR2`) :`2` (`self.COLOR3`) :!type "PrimitiveComponent Object Reference") 0 (select `/Game/enum_color` (`.Color_6_224155634E788CF9DAE571AE1E8B3D0C` (break `/Game/Struct_Ingredient` _struct_type_obj)) :`NewEnumerator0` "/Game/Material/MasterMaterial_FlatShading_Red.MasterMaterial_FlatShading_Red" :`NewEnumerator1` "/Game/Material/MasterMaterial_FlatShading_Green.MasterMaterial_FlatShading_Green" :`NewEnumerator2` "/Game/Material/MasterMaterial_FlatShading_Blue.MasterMaterial_FlatShading_Blue" :!type "MaterialInterface Object Reference")))
      (`self.K2_DestroyActor` _asbp_ingredient))
    (:`CastFailed`
      (`/Engine/EditorBlueprintResources/StandardMacros.IsValid` (`self.CurrentSyringe`)
        (:`Is Not Valid`
          (bind _asbp_syringe (cast `/Game/GPE/Commands/BP_Syringe` OtherActor))
          (if (> (`KismetArrayLibrary.Array_Length` (`self.MixedIngredients`)) 0)
            (set `self.CurrentSyringe` _asbp_syringe)
            (`self.K2_DetachFromActor` _asbp_syringe "KeepWorld" "KeepWorld" "KeepWorld")
            (`PrimitiveComponent.SetSimulatePhysics` (`/Game/GPE/Commands/BP_Syringe.Cylinder1` _asbp_syringe) false)
            (`self.K2_SetActorRotation` _asbp_syringe (struct :`Yaw` 90.0) false)
            (`self.K2_SetActorLocation` _asbp_syringe (`SceneComponent.K2_GetComponentLocation` (`self.Arrow`)) false false)
            (`KismetSystemLibrary.K2_SetTimerDelegate` (delegate `LoadSyringe`) 5.0)))))))

(event `LoadSyringe`
  (`KismetSystemLibrary.PrintString` "Done" true true (struct :`R` 1.0 :`B` 0.01106 :`A` 1.0))
  (set `/Game/GPE/Commands/BP_Syringe.Content` (`self.MixedIngredients`) (`self.CurrentSyringe`))
  (set `self.MixedIngredients` (`|MakeArray`))
  (set `self.CurrentSyringe` null)
  (`PrimitiveComponent.SetMaterial` (`self.COLOR3`) 0 "/Game/SK/Default_Material.Default_Material")
  (`PrimitiveComponent.SetMaterial` (`self.COLOR2`) 0 "/Game/SK/Default_Material.Default_Material")
  (`PrimitiveComponent.SetMaterial` (`self.COLOR1`) 0 "/Game/SK/Default_Material.Default_Material"))

(fn `UserConstructionScript`)