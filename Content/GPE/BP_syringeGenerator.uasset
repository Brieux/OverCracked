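; BP_syringeGenerator is a gameplay element that dispenses BP_Syringe pickups or props at an arrow's transform.
; It spawns one syringe at BeginPlay, then a looping timer periodically checks SpawningCollision for an overlapping syringe.
; When the zone is empty, it spawns a replacement and plays an ejection animation on the skeletal mesh, returning to the looping idle after a delay.
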(event `self.ReceiveBeginPlay`
  (`|SpawnActorFromClass` "/Game/GPE/Commands/BP_Syringe.BP_Syringe_C" (`SceneComponent.K2_GetComponentToWorld` (`self.Arrow`)) "Undefined" "OverrideRootScale" null null)
  (`KismetSystemLibrary.K2_SetTimerDelegate` (delegate `CheckIfSyringe`) 5.0 true))

(event `CheckIfSyringe`
  (if (== (`KismetArrayLibrary.Array_Length` (`PrimitiveComponent.GetOverlappingActors` (`self.SpawningCollision`) "/Game/GPE/Commands/BP_Syringe.BP_Syringe_C")) 0)
    (`|SpawnActorFromClass` "/Game/GPE/Commands/BP_Syringe.BP_Syringe_C" (`SceneComponent.K2_GetComponentToWorld` (`self.Arrow`)) "Undefined" "OverrideRootScale" null null)
    (`SkeletalMeshComponent.PlayAnimation` (`self.SkeletalMesh`) "/Game/Mesh/Animated_Meshes/SeringueOK/anim_seringue_ejection.anim_seringue_ejection" false)
    (`KismetSystemLibrary.Delay` 2.5)
    (`SkeletalMeshComponent.PlayAnimation` (`self.SkeletalMesh`) "/Game/Mesh/Animated_Meshes/SeringueOK/anim_seringue_idle.anim_seringue_idle" true)))

(fn `UserConstructionScript`)