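; BP_TransformationMachine is a machine that converts a BP_Ingredient from one state (solid, liquid or powder) to another, keeping its color.
; An overlapping ingredient matching INType is destroyed and closes a gate; others reaching the open gate are launched along the Arrow.
; A timer then spawns the OUTType ingredient at the Arrow and reopens the gate after a short delay.
; INType also selects the machine's mesh and sounds.
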(event `self.DetectionItem.OnComponentBeginOverlap`
  (params (OverlappedComponent :type "PrimitiveComponent Object Reference") (OtherActor :type "Actor Object Reference") (OtherComp :type "PrimitiveComponent Object Reference") (OtherBodyIndex :type Integer) (bFromSweep :type Boolean) (SweepResult :type "HitResult Structure (by ref)"))
  (`/Engine/EditorBlueprintResources/StandardMacros.Gate` false :!label _label
    (:`Exit`
      (bind _asbp_ingredient (cast `/Game/BP_Ingredient` OtherActor))
      (bind (_struct_type_obj_color _struct_type_obj_state) (break `/Game/Struct_Ingredient` (`/Game/BP_Ingredient.struct_type_obj` _asbp_ingredient)))
      (if (`|EnumEquality` _struct_type_obj_state (`self.INType`))
        (`KismetSystemLibrary.PrintString` "StartTransformation")
        (set `self.RegisteredColor` _struct_type_obj_color)
        (`self.K2_DestroyActor` OtherActor)
        (`|ExecutionSequence`
          (:`then_0`
            (bind _returnvalue (`KismetSystemLibrary.K2_SetTimerDelegate` (delegate `SpawnNewIngredient`) (`self.ConvertionLength`)))
            (set `self.TimerValue` _returnvalue)
            (`GameplayStatics.PlaySound2D` (select `/Game/Enum_State` (`self.INType`) :`NewEnumerator0` "/Game/Sound/SD/MORTIER/SC_Mortier.SC_Mortier" :`NewEnumerator1` "/Game/Sound/SD/MACHINES/SC_Solidification.SC_Solidification" :`NewEnumerator2` "/Game/Sound/SD/CENTRIFUGEUSE/SC_Process.SC_Process" :!type "SoundBase Object Reference") 1.0 1.0 0.0 null null))
          (:`then_1`
            (goto _label :!via `Close`)))
        (else
          (bind _cylinder (`/Game/BP_Ingredient.Cylinder` _asbp_ingredient))
          (`PrimitiveComponent.SetSimulatePhysics` _cylinder true)
          (`PrimitiveComponent.AddImpulse` _cylinder (* (`SceneComponent.GetForwardVector` (`self.Arrow`)) 50000.0) "None" false)
          (`KismetSystemLibrary.PrintString` "Bad"))))))

(event `SpawnNewIngredient`
  (`|SpawnActorFromClass` "/Game/BP_Ingredient.BP_Ingredient_C" (`KismetMathLibrary.MakeTransform` (`SceneComponent.K2_GetComponentLocation` (`self.Arrow`))) "Undefined" "OverrideRootScale" null (select `/Game/Enum_Color` (`self.RegisteredColor`) :`NewEnumerator1` 1 :`NewEnumerator2` 2) (select `/Game/Enum_State` (`self.OUTType`) :`NewEnumerator0` 1 :`NewEnumerator1` 2 :`NewEnumerator2` 3) null)
  (`GameplayStatics.PlaySound2D` (select `/Game/Enum_State` (`self.INType`) :`NewEnumerator0` "/Game/Sound/SD/MORTIER/SC_Mortier.SC_Mortier" :`NewEnumerator1` "/Game/Sound/SD/MACHINES/SC_Solidification.SC_Solidification" :`NewEnumerator2` "/Game/Sound/SD/CENTRIFUGEUSE/SC_Resultat.SC_Resultat" :!type "SoundBase Object Reference") 1.0 1.0 0.0 null null)
  (`KismetSystemLibrary.Delay` 0.5)
  (goto _label :!via `Open`))

(fn `UserConstructionScript`
  (`StaticMeshComponent.SetStaticMesh` (`self.StaticMesh`) (select `/Game/Enum_State` (`self.INType`) :`NewEnumerator1` "/Game/Mesh/Solidification.Solidification" :!type "StaticMesh Object Reference"))
  (`SkinnedMeshComponent.SetSkinnedAssetAndUpdate` (`self.SkeletalMesh`) (select `/Game/Enum_State` (`self.INType`) :`NewEnumerator0` "/Game/Mesh/Animated_Meshes/Mortier/rig_mortier.rig_mortier" :`NewEnumerator2` "/Game/Mesh/Animated_Meshes/Centrifuge/rig_centrifuge.rig_centrifuge" :!type "SkeletalMesh Object Reference") true)
  (if (`|EnumEquality` (`self.INType`) "NewEnumerator2")
    (`SceneComponent.K2_SetRelativeRotation` (`self.SkeletalMesh`) (struct :`Yaw` 180.0) false false)))