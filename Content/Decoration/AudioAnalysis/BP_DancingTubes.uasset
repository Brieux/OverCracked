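; BP_DancingTubes is a decorative prop that bobs and puffs smoke in response to the audio beat intensity.
; On BeginPlay it grabs the first BP_SoundVisualisationProp1 in the level and stores Cube1's base height.
; Each tick it maps that actor's Beatintensity through a curve to drive Cube1's vertical offset and the smoke's SpawnIntensity.
; The construction script gives each tube a random, over-bright smoke color.
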(event `self.ReceiveBeginPlay`
  (bind (_relativelocation_x _relativelocation_y _relativelocation_z) (`KismetMathLibrary.BreakVector` (`SceneComponent.RelativeLocation` (`self.Cube1`))))
  (bind _outactors (`GameplayStatics.GetAllActorsOfClass` "/Game/Decoration/AudioAnalysis/BP_SoundVisualisationProp1.BP_SoundVisualisationProp1_C"))
  (set `self.VisualizerManager` (`|GetArrayItem` _outactors))
  (set `self.GetBasePosition` _relativelocation_z))

(event `self.ReceiveTick`
  (params (DeltaSeconds :type "Float (single-precision)"))
  (bind _returnvalue (`CurveFloat.GetFloatValue` (`self.curveData`) (`/Game/Decoration/AudioAnalysis/BP_SoundVisualisationProp1.Beatintensity` (`self.VisualizerManager`))))
  (`SceneComponent.K2_SetRelativeLocation` (`self.Cube1`) (`KismetMathLibrary.MakeVector` 0.0 0.0 (+ (* _returnvalue 20.0) (`self.GetBasePosition`))) false false)
  (`NiagaraComponent.SetVariableFloat` (`self.NS_TubeSmoke`) "SpawnIntensity" (* _returnvalue 100.0)))

(fn `UserConstructionScript`
  (`NiagaraComponent.SetVariableLinearColor` (`self.NS_TubeSmoke`) "SmokeColor" (make `LinearColor` (* (`KismetMathLibrary.RandomFloat`) 10.0) (* (`KismetMathLibrary.RandomFloat`) 10.0) (* (`KismetMathLibrary.RandomFloat`) 10.0) 0.6)))