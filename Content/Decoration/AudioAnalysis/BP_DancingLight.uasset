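; BP_DancingLight is a decorative prop whose material reacts to music beat intensity.
; Construction creates a dynamic Metal material instance on the second material slot of Cube1.
; BeginPlay caches the first BP_SoundVisualisationProp1 as its manager and stores the cube's base height, which is never used here.
; Each Tick maps the manager's Beatintensity through a curve and writes the inverted value to the "Color" scalar parameter.
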(event `self.ReceiveBeginPlay`
  (bind (_relativelocation_x _relativelocation_y _relativelocation_z) (`KismetMathLibrary.BreakVector` (`SceneComponent.RelativeLocation` (`self.Cube1`))))
  (bind _outactors (`GameplayStatics.GetAllActorsOfClass` "/Game/Decoration/AudioAnalysis/BP_SoundVisualisationProp1.BP_SoundVisualisationProp1_C"))
  (set `self.VisualizerManager` (`|GetArrayItem` _outactors))
  (set `self.GetBasePosition` _relativelocation_z))

(event `self.ReceiveTick`
  (params (DeltaSeconds :type "Float (single-precision)"))
  (`MaterialInstanceDynamic.SetScalarParameterValue` (`self.MaterialAlteration`) "Color" (- 1.0 (`CurveFloat.GetFloatValue` (`self.curveData`) (`/Game/Decoration/AudioAnalysis/BP_SoundVisualisationProp1.Beatintensity` (`self.VisualizerManager`))))))

(fn `UserConstructionScript`
  (bind _returnvalue (`PrimitiveComponent.CreateDynamicMaterialInstance` (`self.Cube1`) 1 "/Game/Mesh/metal.metal" "None"))
  (set `self.MaterialAlteration` _returnvalue))