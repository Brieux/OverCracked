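; BP_SoundVisualisationProp1 is a decoration prop that plays a sound and tracks its loudness for audio visualisation.
; The construction script assigns the BeatAnalyser's sound to the BeatAudio component and caches its duration.
; During playback, the playback percent becomes a timestamp for sampling normalized loudness from the analyser into Beatintensity.
; The audio restarts from the beginning whenever it finishes, and nothing in these graphs consumes Beatintensity.
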(event `self.BeatAudio.OnAudioFinished`
  ;[1 1 1] Reset audio/changeTrack
  (`AudioComponent.Play` (`self.BeatAudio`) 0.0))

(event `self.BeatAudio.OnAudioPlaybackPercent`
  (params (PlayingSoundWave :type "SoundWave Object Reference") (PlaybackPercent :type "Float (single-precision)"))
  (set `self.Beatintensity` (`LoudnessNRT.GetNormalizedLoudnessAtTime` (`self.BeatAnalyser`) (* PlaybackPercent (`self.Length`)))))

(fn `UserConstructionScript`
  (bind _sound (`AudioAnalyzerNRT.Sound` (`self.BeatAnalyser`)))
  (`AudioComponent.SetSound` (`self.BeatAudio`) _sound)
  (set `self.Length` (`SoundBase.Duration` _sound)))