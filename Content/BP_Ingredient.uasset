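; BP_Ingredient is a pickup ingredient with a color and a solid, liquid or powder state that the top-down character can take.
; The construction script builds its ingredient struct from the chosen color and a forced or random state, and picks the mesh by color.
; Box overlaps set or clear the character's take target.
; Ciao disables physics, teleports it to a fixed position and calls Collected, while Shake plays a throttled state-specific sound.
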(event `self.Box.OnComponentBeginOverlap`
  (params (OverlappedComponent :type "PrimitiveComponent Object Reference") (OtherActor :type "Actor Object Reference") (OtherComp :type "PrimitiveComponent Object Reference") (OtherBodyIndex :type Integer) (bFromSweep :type Boolean) (SweepResult :type "HitResult Structure (by ref)"))
  (bind _asbp_top_down_character (cast `/Game/TopDown/Blueprints/BP_TopDownCharacter` OtherActor))
  (set `/Game/TopDown/Blueprints/BP_TopDownCharacter.CanTakeSomething` true _asbp_top_down_character)
  (set `/Game/TopDown/Blueprints/BP_TopDownCharacter.CanTakeThis` self _asbp_top_down_character))

(event `self.Box.OnComponentEndOverlap`
  (params (OverlappedComponent :type "PrimitiveComponent Object Reference") (OtherActor :type "Actor Object Reference") (OtherComp :type "PrimitiveComponent Object Reference") (OtherBodyIndex :type Integer))
  (bind _asbp_top_down_character (cast `/Game/TopDown/Blueprints/BP_TopDownCharacter` OtherActor))
  (set `/Game/TopDown/Blueprints/BP_TopDownCharacter.CanTakeSomething` false _asbp_top_down_character)
  (set `/Game/TopDown/Blueprints/BP_TopDownCharacter.CanTakeThis` null _asbp_top_down_character))

(event `/Game/GPE/BPI_Grabbable.Ciao`
  (params (PlayerHolding :type "/Game/TopDown/Blueprints/BP_TopDownCharacter Object Reference"))
  (bind (_returnvalue_location _returnvalue_rotation _returnvalue_scale) (`KismetMathLibrary.BreakTransform` (`self.GetTransform`)))
  (`PrimitiveComponent.SetSimulatePhysics` (`self.Cylinder`) false)
  (`self.K2_SetActorTransform` (`KismetMathLibrary.MakeTransform` (3000.0 4000.0 -130.0) _returnvalue_rotation _returnvalue_scale))
  (`self.Collected`))

(event `Shake`
  (`/Engine/EditorBlueprintResources/StandardMacros.DoOnce` false :!label _label
    (:`Completed`
      (`GameplayStatics.SpawnSound2D` (select `/Game/Enum_State` (`.State_7_2AEC6E204EC55F64B9581D9233582410` (break `/Game/Struct_Ingredient` (`self.struct_type_obj`))) :`NewEnumerator0` "/Game/Sounds/SOLIDE/SD_flacon_solide_1_Cue.SD_flacon_solide_1_Cue" :`NewEnumerator1` "/Game/Sounds/LIQUIDE/SD_flacon_liquide_1_Cue.SD_flacon_liquide_1_Cue" :`NewEnumerator2` "/Game/Sounds/POUDREUX/SD_flacon_poudreux_1_Cue.SD_flacon_poudreux_1_Cue" :!type "SoundBase Object Reference") 1.0 1.0 0.0 null)
      (`KismetSystemLibrary.Delay` 0.2)
      (goto _label :!via `Reset`))))

(fn `UserConstructionScript`
  (bind _returnvalue (select `int` (`self.InitiatedColorType`) :`0` "NewEnumerator0" :`1` "NewEnumerator1" :`2` "NewEnumerator2" :!type "/Game/Enum_Color Enum"))
  (set `self.struct_type_obj` (make `/Game/Struct_Ingredient` _returnvalue (select `int` (`self.ForcedValue`) :`0` (select `int` (`KismetMathLibrary.RandomInteger` 3) :`0` "NewEnumerator0" :`1` "NewEnumerator1" :`2` "NewEnumerator2" :!type "/Game/Enum_State Enum") :`1` "NewEnumerator0" :`2` "NewEnumerator1" :`3` "NewEnumerator2")))
  (`StaticMeshComponent.SetStaticMesh` (`self.StaticMesh`) (select `/Game/Enum_Color` _returnvalue :`NewEnumerator0` "/Game/Mesh/SM_Ingredient_R.SM_Ingredient_R" :`NewEnumerator1` "/Game/Mesh/SM_Ingredient_Y.SM_Ingredient_Y" :`NewEnumerator2` "/Game/Mesh/SM_Ingredient_B.SM_Ingredient_B" :!type "StaticMesh Object Reference")))